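; Health pickup Blueprint that restores health to the player's ShooterCharacter_BP.
; Its Healing event casts the first player pawn to ShooterCharacter_BP and adds HealingAmount to Health, capped at MaxHealth.
; Nothing in its own graphs calls Healing, and BeginPlay and the construction script are empty.
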(event EventBeginPlay)

(event EventHealing
  (bind _asshooter_character_bp (Utilities|Casting|CastToShooterCharacter_BP (Game|Player|GetPlayerPawn 0)))
  (if (>= (+ (Variables|/Script/Shooter.ShooterCharacter|GetHealth _asshooter_character_bp) (Variables|Default|GetHealingAmount self)) (Variables|/Script/Shooter.ShooterCharacter|GetMaxHealth _asshooter_character_bp))
    (Variables|/Script/Shooter.ShooterCharacter|SetHealth _asshooter_character_bp (Variables|/Script/Shooter.ShooterCharacter|GetMaxHealth _asshooter_character_bp))
    (else
      (Variables|/Script/Shooter.ShooterCharacter|SetHealth _asshooter_character_bp (+ (Variables|/Script/Shooter.ShooterCharacter|GetHealth _asshooter_character_bp) (Variables|Default|GetHealingAmount self))))))

(fn ConstructionScript)